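; BP_PlayerB is the Blueprint for player B, relaying that player's input and triggering the level change to the ending.
; Forward and right inputs call MoveForward and Turn, while interact inputs call BOnInteract and BDeInteract, none of which are defined in this graph.
; Tick polls BState every frame and opens EndingMap by name once it equals BEnd.
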(event EventPlayerBInteract
  ;[1 1 1] 입력값 받기
  (Class|PlayerB|BonInteract))

(event Collision|EventActorBeginOverlap
  (params (OtherActor :type Actor%20Object%20Reference)))

(event EventTick
  (params (DeltaSeconds :type Float%20%28single-precision%29))
  (if (Utilities|Enum|Equal(Enum) (Variables|Default|GetbState) "B_End")
    (Game|OpenLevel(byName) "EndingMap")))

(event EventPlayerBDeInteract
  ;[1 1 1] 입력값 받기
  (Class|PlayerB|BDeInteract))

(event EventPlayerBForwardInput
  (params (value :type Float%20%28single-precision%29))
  ;[1 1 1] 입력값 받기
  (Class|PlayerB|MoveForward value))

(event EventPlayerBRightInput
  (params (value :type Float%20%28single-precision%29))
  ;[1 1 1] 입력값 받기
  (Class|PlayerB|Turn value))

(event EventBeginPlay)

(fn ConstructionScript)