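; BP_PlayerA receives input and relays it to other actors, acting as the control hub for Player B and the CCTV.
; Move, turn and interact press/release inputs are forwarded to BP_PlayerB, while the CCTV turn axis goes to BP_CCTV.
; Each event looks up its target with GetActorOfClass on every call, with no cached reference, and passes the value to that actor's handler function.
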(event Collision|EventActorBeginOverlap
  (params (OtherActor :type Actor%20Object%20Reference)))

(event Input|ActionEvents|InputActionTestInteract
  (params (Key :type Key%20Structure :default "None"))
  ;[1 1 1] Player B 상호작용 입력값 전달
  (:Pressed
    (bind _returnvalue (Actor|GetActorOfClass "/Game/Blueprint/ControllBlueprint/BP_PlayerB.BP_PlayerB_C"))
    (Default|PlayerBInteract _returnvalue))
  (:Released
    (bind _returnvalue_2 (Actor|GetActorOfClass "/Game/Blueprint/ControllBlueprint/BP_PlayerB.BP_PlayerB_C"))
    (Default|PlayerBDeInteract _returnvalue_2)))

(event Input|AxisEvents|InputAxisPlayerBMoveForward
  (params (AxisValue :type Float%20%28single-precision%29))
  ;[1 1 1] Player B에게 이동 입력값 전달
  (bind _returnvalue (Actor|GetActorOfClass "/Game/Blueprint/ControllBlueprint/BP_PlayerB.BP_PlayerB_C"))
  (Default|PlayerBForwardInput _returnvalue AxisValue))

(event Input|AxisEvents|InputAxisCCTVTurn
  (params (AxisValue :type Float%20%28single-precision%29))
  (bind _returnvalue (Actor|GetActorOfClass "/Game/Blueprint/ControllBlueprint/BP_CCTV.BP_CCTV_C"))
  (Default|CCTVRightInput _returnvalue AxisValue))

(event Input|AxisEvents|InputAxisPlayerBTurn
  (params (AxisValue :type Float%20%28single-precision%29))
  ;[1 1 1] Player B에게 이동 입력값 전달
  (bind _returnvalue (Actor|GetActorOfClass "/Game/Blueprint/ControllBlueprint/BP_PlayerB.BP_PlayerB_C"))
  (Default|PlayerBRightInput _returnvalue AxisValue))

(fn ConstructionScript)